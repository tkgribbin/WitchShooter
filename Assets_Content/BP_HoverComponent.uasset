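; BP_HoverComponent is a hover component that pushes its owning BP_Projectile_Base away from surfaces beneath it.
; Each tick it line-traces along its negative up vector for HoverHeight, with debug drawing on.
; On a hit, a spring-damper force from compression and its rate of change (Suspension, Damping) is applied to the projectile's root primitive at the component's location.
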(event `self.ReceiveBeginPlay`
  (bind _asbp_projectile_base (cast `/Game/Weapons/BP_Projectile_Base` (`self.GetOwner`)))
  (set `self.ParentProjectile` _asbp_projectile_base))

(event `self.ReceiveTick`
  (params (DeltaSeconds :type "Float (single-precision)"))
  (bind _returnvalue (`self.K2_GetComponentLocation`))
  (`/Engine/EditorBlueprintResources/StandardMacros.IsValid` (`self.ParentProjectile`)
    (:`Is Valid`
      (bind (_outhit _returnvalue_2) (`KismetSystemLibrary.LineTraceSingle` :`Start` _returnvalue :`End` (- _returnvalue (* (`self.GetUpVector`) (`self.HoverHeight`))) :`TraceChannel` "TraceTypeQuery1" :`DrawDebugType` "ForOneFrame"))
      (if _returnvalue_2
        (bind _output_get (set `self.HoverDelta` (- (`self.HoverHeight`) (`.Distance` (`GameplayStatics.BreakHitResult` _outhit)))))
        (`PrimitiveComponent.AddForceAtLocation` (cast `PrimitiveComponent` (`Actor.RootComponent` (`self.ParentProjectile`)) :!pure true) (* (`self.GetUpVector`) (+ (* (/ (- _output_get (`self.PreviousHoverDelta`)) (`GameplayStatics.GetWorldDeltaSeconds`)) (`self.Damping`)) (* _output_get (`self.Suspension`)))) (`self.K2_GetComponentLocation`) "None")
        (set `self.PreviousHoverDelta` (`self.HoverDelta`))))))